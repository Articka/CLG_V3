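; HUD is a Blueprint of helper functions that splits underscore-delimited strings into lists of action names.
; GetAllAction builds each name character by character and appends it to the target array at every underscore, so text after the last underscore is not added.
; AddButton and AddNumberOfItem are empty stubs.
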(fn `AddButton`)

(fn `AddNumberOfItem`)

(fn `GetAllAction`
  (params (SourceString :type String) (TargetArray :type "Array of String (by ref)"))
  (locals (NewActionName :type String))
  (set `local.NewActionName` "")
  (for _array_element (`KismetStringLibrary.GetCharacterArrayFromString` SourceString)
    (if (not (`KismetStringLibrary.EqualEqual_StrStr` _array_element "_"))
      (set `local.NewActionName` (`KismetStringLibrary.Concat_StrStr` (`local.NewActionName`) _array_element))
      (else
        (`KismetArrayLibrary.Array_Add` TargetArray (`local.NewActionName`))
        (set `local.NewActionName` "")))))