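; Usable storage container that holds pickable items and opens for the LittleGirl_2D character when used.
; On BeginPlay it spawns each Container entry as a Pickable flagged as in storage, then sets its weight and count using an item data table keyed by class name.
; On Use it passes the item list to the character's Storage and opens it, while SetItem lets that list be replaced.
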(event `self.ReceiveBeginPlay`
  (for _array_element (`self.Container`)
    (bind (_itemtostore _numberofitem) (break `/Game/Blueprint/Structure/Storage` _array_element))
    (bind _returnvalue (`|SpawnActorFromClass` _itemtostore (`KismetMathLibrary.MakeTransform` (0.0 0.0 0.0)) "Undefined" "OverrideRootScale" null null))
    (bind _aspickable (cast `/Game/Blueprint/Usable_Item/Pickable` _returnvalue))
    (`/Game/Blueprint/Usable_Item/Pickable.SetInStorage` _aspickable true)
    (bind _nameofclassactor (`/Game/Blueprint/Function/GetNameOfClass.GetNameOfClass` _returnvalue))
    (bind _returnvalue_2 (`|GetDataTableRow` "/Game/Blueprint/Datatable/ItemInformation_-_Feuille_1__1_.ItemInformation_-_Feuille_1__1_" _nameofclassactor)
      (:`then`
        (`/Game/Blueprint/Usable_Item/Pickable.CreateNewItem` _aspickable (`.Weight_2_ABCA71D441418047A79A818B8C81A5BA` (break `/Game/Blueprint/Structure/Database/ItemInformation` _returnvalue_2)) _numberofitem)
        (`KismetArrayLibrary.Array_Add` (`self.Item`) _returnvalue)))))

(event `self.Use`
  (params (ActorUse :type "Actor Object Reference"))
  (bind _aslittle_girl_2d (cast `/Game/Blueprint/Character/Player/2D/LittleGirl_2D` ActorUse))
  (`/Game/Blueprint/HUD/Stockage/Storage_HUD.CreateStorage` (`/Game/Blueprint/Character/Player/2D/LittleGirl_2D.Storage` _aslittle_girl_2d) (`self.Item`))
  (`/Game/Blueprint/Character/Player/2D/LittleGirl_2D.OpenStorage` _aslittle_girl_2d self))

(fn `SetItem`
  (params (Item :type "Array of Actor Object Reference"))
  (set `self.Item` Item)
  (return))

(fn `UserConstructionScript`
  (`parent.UserConstructionScript`))