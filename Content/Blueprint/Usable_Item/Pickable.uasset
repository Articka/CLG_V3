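; Base pickable item actor for the LittleGirl_2D player's inventory and storage, with an empty override hook for each item's use effect.
; Pickup checks slot and weight limits, then merges same-class stacks or keeps the actor, moved to world origin.
; Partial pickup spawns a same-class actor for new stacks, reading weight from a data table by class name.
; Using an item decrements its count, then updates inventory or storage, or destroys the depleted world actor.
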(event `self.Use`
  (params (ActorUse :type "Actor Object Reference"))
  (`self.UseItem`))

(fn `CheckIfItemCanAdd`
  (params (AddNew :type Boolean) (WeightOfItem :type "Float (double-precision)") (NumberOfItem :type Integer) (PlayerInventory :type "/Game/Blueprint/Structure/Inventory Structure"))
  (returns (`CanAdd ?` :type Boolean))
  (bind (_maximumofdifferentobject _maximumofweight _actualweight _itemactor) (break `/Game/Blueprint/Structure/Inventory` PlayerInventory))
  (bind _returnvalue (+ (* NumberOfItem WeightOfItem) _actualweight))
  (if AddNew
    (if (<= (+ (`KismetArrayLibrary.Array_Length` _itemactor) 1) _maximumofdifferentobject)
      _
      (else
        (`KismetSystemLibrary.PrintString` "Ne peux pas prendre d'objet différents en plus.")
        (return false))))
  (if (not (< _maximumofweight _returnvalue))
    (bind _aslittle_girl_2d (cast `/Game/Blueprint/Character/Player/2D/LittleGirl_2D` (`GameplayStatics.GetPlayerCharacter` 0)))
    (bind (_inventory_maximumofdifferentobject _inventory_maximumofweight _inventory_actualweight _inventory_itemactor) (break `/Game/Blueprint/Structure/Inventory` (`/Game/Blueprint/Character/Player/2D/LittleGirl_2D.Inventory` _aslittle_girl_2d)))
    (`/Game/Blueprint/Character/Player/2D/LittleGirl_2D.Inventory_SetInventory` _aslittle_girl_2d _inventory_maximumofdifferentobject _inventory_maximumofweight _returnvalue _inventory_itemactor)
    (return true)
    (else
      (`KismetSystemLibrary.PrintString` "Ne peux pas prendre d'objet car ça serait trop lourd.")
      (return false))))

(fn `CreateNewItem`
  (params (Weight :type "Float (double-precision)") (NumberOfItem :type Integer))
  ;[1 1 1] Be careful, set sprite as not here :'(
  (set `self.Weight` Weight)
  (set `self.NumberOfItem` NumberOfItem)
  (return))

(fn `DestroySelf`
  (`self.K2_DestroyActor`)
  (return))

(fn `GetNumberOfItem`
  (returns (GetNumberOfItem :type Integer))
  (return (`self.NumberOfItem`)))

(fn `ModificateNumberOfItem`
  (params (AddOrRemove :type Integer))
  (set `self.NumberOfItem` (+ AddOrRemove (`self.NumberOfItem`)))
  (`self.SetInventoryAfterItemUse`)
  (return))

(fn `OVERRIDE_USE`)

(fn `PickUp`
  (params (PlayerInventory :type "/Game/Blueprint/Structure/Inventory Structure"))
  (returns (Return :type Boolean))
  (bind (_maximumofdifferentobject _maximumofweight _actualweight _itemactor) (break `/Game/Blueprint/Structure/Inventory` PlayerInventory))
  (if (== (`KismetArrayLibrary.Array_Length` _itemactor) 0)
    ;[1 1 1] Si rien dans l'inventaire
    (bind _canadd__ (`self.CheckIfItemCanAdd` true (`self.Weight`) (`self.NumberOfItem`) PlayerInventory))
    (if _canadd__
      (bind _aslittle_girl_2d (cast `/Game/Blueprint/Character/Player/2D/LittleGirl_2D` (`GameplayStatics.GetPlayerCharacter` 0)))
      (`/Game/Blueprint/Character/Player/2D/LittleGirl_2D.Inventory_AddItemInInventory` _aslittle_girl_2d self)
      ;;[1 1 1] "Teleport" item
      (`self.K2_SetActorLocation` (0.0 0.0 0.0))
      (set `self.InInventory` true)
      (if (`self.inStorage`)
        (set `self.inStorage` false))
      (return true)
      (else
        (return false)))
    (else
      ;[1 1 1] Si l'objet est déjà dans l'inventaire
      (set `self.TestIfObjetAsAllreadyInInventory` false)
      (for _array_element _itemactor
        (bind _nameofclassactor (`/Game/Blueprint/Function/GetNameOfClass.GetNameOfClass` _array_element))
        (bind _nameofclassactor_2 (`/Game/Blueprint/Function/GetNameOfClass.GetNameOfClass` self))
        (if (== _nameofclassactor_2 _nameofclassactor)
          ;;[1 1 1] Objet qui existe déjà dans l'inventaire
          (bind _canadd___2 (`self.CheckIfItemCanAdd` false (`self.Weight`) (`self.NumberOfItem`) PlayerInventory))
          (if _canadd___2
            (bind _aspickable (cast `/Game/Blueprint/Usable_Item/Pickable` _array_element))
            (`self.ModificateNumberOfItem` _aspickable (`self.NumberOfItem`))
            (`KismetSystemLibrary.PrintString` "Object in inventory and the number of this item are increase.")
            (`self.DestroySelf`)
            (set `self.TestIfObjetAsAllreadyInInventory` true)
            (return true)
            (else
              (return false)))))
      ;[1 1 1] Nouvelle objet dans l'inventaire
      (if (not (`self.TestIfObjetAsAllreadyInInventory`))
        (bind _canadd___3 (`self.CheckIfItemCanAdd` true (`self.Weight`) (`self.NumberOfItem`) PlayerInventory))
        (if _canadd___3
          ;;[1 1 1] Objet qui n'existe pas dans l'inventaire et qui est ajouté
          (bind _aslittle_girl_2d_2 (cast `/Game/Blueprint/Character/Player/2D/LittleGirl_2D` (`GameplayStatics.GetPlayerCharacter` 0)))
          (`/Game/Blueprint/Character/Player/2D/LittleGirl_2D.Inventory_AddItemInInventory` _aslittle_girl_2d_2 self)
          ;;;[1 1 1] "Teleport" item
          (`self.K2_SetActorLocation` (0.0 0.0 0.0))
          (set `self.InInventory` true)
          (if (`self.inStorage`)
            (set `self.inStorage` false))
          (return true)
          (else
            _)))
      (return false))))

(fn `PickUp_Number`
  (params (Inventory :type "/Game/Blueprint/Structure/Inventory Structure (by ref)") (NumberOfTakingItem :type Integer))
  (returns (Return :type Boolean))
  (bind (_maximumofdifferentobject _maximumofweight _actualweight _itemactor) (break `/Game/Blueprint/Structure/Inventory` Inventory))
  (if (== (`KismetArrayLibrary.Array_Length` _itemactor) 0)
    ;[1 1 1] Si rien dans l'inventaire
    (bind _canadd__ (`self.CheckIfItemCanAdd` true (`self.Weight`) NumberOfTakingItem Inventory))
    (if _canadd__
      (bind _aslittle_girl_2d (cast `/Game/Blueprint/Character/Player/2D/LittleGirl_2D` (`GameplayStatics.GetPlayerCharacter` 0)))
      (set `self.NumberOfItem` (- (`self.NumberOfItem`) NumberOfTakingItem))
      ;;[1 1 1] Create new item
      (bind _returnvalue (`|SpawnActorFromClass` (`GameplayStatics.GetObjectClass` self) (`KismetMathLibrary.MakeTransform` (0.0 0.0 0.0)) "Undefined" "OverrideRootScale" null null))
      (bind _nameofclassactor (`/Game/Blueprint/Function/GetNameOfClass.GetNameOfClass` _returnvalue))
      (bind _returnvalue_2 (`|GetDataTableRow` "/Game/Blueprint/Datatable/ItemInformation_-_Feuille_1__1_.ItemInformation_-_Feuille_1__1_" _nameofclassactor)
        (:`then`
          (`self.CreateNewItem` _returnvalue (`.Weight_2_ABCA71D441418047A79A818B8C81A5BA` (break `/Game/Blueprint/Structure/Database/ItemInformation` _returnvalue_2)) NumberOfTakingItem)
          (set `/Game/Blueprint/Usable_Item/Pickable.InInventory` true _returnvalue)
          (`/Game/Blueprint/Character/Player/2D/LittleGirl_2D.Inventory_AddItemInInventory_Number` _aslittle_girl_2d _returnvalue)
          (return true)))
      (else
        (return false)))
    (else
      ;[1 1 1] Si l'objet est déjà dans l'inventaire
      (set `self.TestIfObjetAsAllreadyInInventory` false)
      (for _array_element _itemactor
        (bind _aspickable (cast `/Game/Blueprint/Usable_Item/Pickable` _array_element))
        (bind _nameofclassactor_2 (`/Game/Blueprint/Function/GetNameOfClass.GetNameOfClass` _aspickable))
        (bind _nameofclassactor_3 (`/Game/Blueprint/Function/GetNameOfClass.GetNameOfClass` self))
        (if (== _nameofclassactor_2 _nameofclassactor_3)
          ;;[1 1 1] Objet qui existe déjà dans l'inventaire
          (bind _canadd___2 (`self.CheckIfItemCanAdd` false (`self.Weight`) NumberOfTakingItem Inventory))
          (if _canadd___2
            (bind _aspickable_2 (cast `/Game/Blueprint/Usable_Item/Pickable` _array_element))
            (`self.ModificateNumberOfItem` _aspickable_2 NumberOfTakingItem)
            (`KismetSystemLibrary.PrintString` "Object in inventory and the number of this item are increase.")
            (bind _output_get (set `self.NumberOfItem` (- (`self.NumberOfItem`) NumberOfTakingItem)))
            (if (== _output_get 0)
              (`self.DestroySelf`)
              (set `self.TestIfObjetAsAllreadyInInventory` true)
              (else
                (set `self.TestIfObjetAsAllreadyInInventory` true)))
            (return true)
            (else
              (return false)))))
      ;[1 1 1] Nouvelle objet dans l'inventaire
      (if (not (`self.TestIfObjetAsAllreadyInInventory`))
        (bind _canadd___3 (`self.CheckIfItemCanAdd` true (`self.Weight`) NumberOfTakingItem))
        (if _canadd___3
          ;;[1 1 1] Objet qui n'existe pas dans l'inventaire et qui est ajouté
          (bind _aslittle_girl_2d_2 (cast `/Game/Blueprint/Character/Player/2D/LittleGirl_2D` (`GameplayStatics.GetPlayerCharacter` 0)))
          (set `self.NumberOfItem` (- (`self.NumberOfItem`) NumberOfTakingItem))
          ;;[1 1 1] Create new item
          (bind _returnvalue_3 (`|SpawnActorFromClass` (`GameplayStatics.GetObjectClass` self) (`KismetMathLibrary.MakeTransform` (0.0 0.0 0.0)) "Undefined" "OverrideRootScale" null null))
          (bind _nameofclassactor_4 (`/Game/Blueprint/Function/GetNameOfClass.GetNameOfClass` _returnvalue_3))
          (set `/Game/Blueprint/Usable_Item/Pickable.InInventory` true _returnvalue_3)
          (bind _returnvalue_4 (`|GetDataTableRow` "/Game/Blueprint/Datatable/ItemInformation_-_Feuille_1__1_.ItemInformation_-_Feuille_1__1_" _nameofclassactor_4)
            (:`then`
              (`self.CreateNewItem` _returnvalue_3 (`.Weight_2_ABCA71D441418047A79A818B8C81A5BA` (break `/Game/Blueprint/Structure/Database/ItemInformation` _returnvalue_4)) NumberOfTakingItem)
              (`/Game/Blueprint/Character/Player/2D/LittleGirl_2D.Inventory_AddItemInInventory_Number` _aslittle_girl_2d_2 _returnvalue_3)
              (return true)))
          (else
            _)))
      (return false))))

(fn `SetInStorage`
  (params (InStorage :type Boolean))
  (set `self.InStorage` InStorage)
  (return))

(fn `SetInventoryAfterItemUse`
  (locals (Destroy :type Boolean) (WeightAdd :type "Float (double-precision)"))
  (bind _aslittle_girl_2d (cast `/Game/Blueprint/Character/Player/2D/LittleGirl_2D` (`GameplayStatics.GetPlayerCharacter` 0)))
  (bind (_inventory_maximumofdifferentobject _inventory_maximumofweight _inventory_actualweight _inventory_itemactor) (break `/Game/Blueprint/Structure/Inventory` (`/Game/Blueprint/Character/Player/2D/LittleGirl_2D.Inventory` _aslittle_girl_2d)))
  (for _array_element _inventory_itemactor
    (bind _aspickable (cast `/Game/Blueprint/Usable_Item/Pickable` _array_element))
    (bind _numberofitem (`/Game/Blueprint/Usable_Item/Pickable.NumberOfItem` _aspickable))
    (if (== _numberofitem 0)
      (bind _returnvalue (`KismetArrayLibrary.Array_RemoveItem` _inventory_itemactor _array_element))
      (set `local.Destroy` _returnvalue))
    (set `local.WeightAdd` (+ (* _numberofitem (`/Game/Blueprint/Usable_Item/Pickable.Weight` _aspickable)) (`local.WeightAdd`)))
    (if (`local.Destroy`)
      (`self.DestroySelf` _aspickable)))
  (bind (_inventory_maximumofdifferentobject_2 _inventory_maximumofweight_2 _inventory_actualweight_2 _inventory_itemactor_2) (break `/Game/Blueprint/Structure/Inventory` (`/Game/Blueprint/Character/Player/2D/LittleGirl_2D.Inventory` _aslittle_girl_2d)))
  (`/Game/Blueprint/Character/Player/2D/LittleGirl_2D.Inventory_SetInventory` _aslittle_girl_2d _inventory_maximumofdifferentobject_2 _inventory_maximumofweight_2 (`local.WeightAdd`) _inventory_itemactor_2)
  (`/Game/Blueprint/HUD/Inventory/Inventory_HUD.RefreshInfo` (`/Game/Blueprint/Character/Player/2D/LittleGirl_2D.InventoryHUD` _aslittle_girl_2d)))

(fn `SetStorageAfterUse`
  (locals (Destroy :type Boolean))
  (bind _aslittle_girl_2d (cast `/Game/Blueprint/Character/Player/2D/LittleGirl_2D` (`GameplayStatics.GetPlayerCharacter` 0)))
  (bind _asstorage (cast `/Game/Blueprint/Usable_Item/Storage` (`/Game/Blueprint/Character/Player/2D/LittleGirl_2D.Storage_Ref` _aslittle_girl_2d)))
  (bind _item (`/Game/Blueprint/Usable_Item/Storage.Item` _asstorage))
  (for _array_element _item
    (bind _aspickable (cast `/Game/Blueprint/Usable_Item/Pickable` _array_element))
    (bind _getnumberofitem (`self.GetNumberOfItem` _aspickable))
    (if (== _getnumberofitem 0)
      (bind _returnvalue (`KismetArrayLibrary.Array_RemoveItem` _item _array_element))
      (set `local.Destroy` _returnvalue))
    (`/Game/Blueprint/Usable_Item/Storage.SetItem` _asstorage _item)
    (if (`local.Destroy`)
      (`self.DestroySelf`)))
  (bind _storage (`/Game/Blueprint/Character/Player/2D/LittleGirl_2D.Storage` _aslittle_girl_2d))
  (`/Game/Blueprint/HUD/Stockage/Storage_HUD.Destruct_Call` _storage)
  (`/Game/Blueprint/HUD/Stockage/Storage_HUD.CreateStorage` _storage (`/Game/Blueprint/Usable_Item/Storage.Item` _asstorage))
  (return))

(fn `UseItem`
  (bind _result (`/Engine/EditorBlueprintResources/StandardMacros.DecrementInt` (`self.NumberOfItem`))
    (:`  `
      (`self.OVERRIDE_USE`)
      (if (`self.InInventory`)
        (`self.SetInventoryAfterItemUse`)
        (elif (`self.inStorage`)
          (`self.SetStorageAfterUse`)
          (elif (== _result 0)
            (`self.K2_DestroyActor`)
            ;[1 1 1] Reset all truc interactible
            (bind _aslittle_girl_2d (cast `/Game/Blueprint/Character/Player/2D/LittleGirl_2D` (`GameplayStatics.GetPlayerCharacter` 0)))
            (set `/Game/Blueprint/Character/Player/2D/LittleGirl_2D.CanInteractible` false _aslittle_girl_2d)
            (set `/Game/Blueprint/Character/Player/2D/LittleGirl_2D.isOnObject` null _aslittle_girl_2d)
            (set `/Game/Blueprint/Character/Player/2D/LittleGirl_2D.TouchActor` null _aslittle_girl_2d)
            (`/Game/Blueprint/Character/Player/2D/LittleGirl_2D.RemoveFromParentMenuAction` _aslittle_girl_2d)))))))

(fn `UserConstructionScript`
  (`parent.UserConstructionScript`))