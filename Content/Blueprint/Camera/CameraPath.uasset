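; CameraPath is a spline camera-rail Blueprint whose active state is toggled as the LittleGirl 2D player character moves through trigger boxes.
; Overlapping either of its two boxes deactivates every CameraPath in the level, then marks this one active, keeping one path active at a time.
; Logic to glide the cine camera to the closest spline point and aim it at the girl exists but is disconnected, and Tick is empty.
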(event `self.ReceiveBeginPlay`
  (bind _aslittle_girl_2d_newpathfinding (cast `/Game/Blueprint/Character/Player/2D/LittleGirl_2D_Newpathfinding` (`GameplayStatics.GetPlayerCharacter` 0)))
  (set `self.LittleGirl` _aslittle_girl_2d_newpathfinding))

(event `self.ReceiveTick`
  (params (DeltaSeconds :type "Float (single-precision)")))

(event `Deactivate isActive`
  (set `self.isActive` false))

(event `self.SecondBoxRef.OnActorBeginOverlap`
  (params (OverlappedActor :type "Actor Object Reference") (OtherActor :type "Actor Object Reference"))
  (cast `/Game/Blueprint/Character/Player/2D/LittleGirl_2D_Newpathfinding` OtherActor)
  (bind _outactors (`GameplayStatics.GetAllActorsOfClass` "CameraPath_C" :!label _label))
  (for _array_element _outactors
    (`self.Deactivate isActive` _array_element))
  (set `self.isActive` true))

(event `self.BoxReference.OnActorBeginOverlap`
  (params (OverlappedActor :type "Actor Object Reference") (OtherActor :type "Actor Object Reference"))
  (cast `/Game/Blueprint/Character/Player/2D/LittleGirl_2D_Newpathfinding` OtherActor)
  (goto _label))

(fn `UserConstructionScript`)